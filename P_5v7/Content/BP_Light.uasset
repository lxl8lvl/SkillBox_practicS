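; Blinking point light Blueprint that flashes a set number of times and then stays off.
; BeginPlay runs a latent loop that hides the light for a configurable delay, shows it for one second and increments a counter until it matches SetCounter.
; The construction script applies the chosen color to the light, and Tick prints the counter every frame as debug output.
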(event EventBeginPlay
  (bind _pointlight (Variables|Default|GetPointLight))
  (if (== (Variables|Default|GetSet_Counter) (Variables|Default|GetCounter)) :!label _label
    (Rendering|SetVisibility _pointlight false false)
    (else
      (Rendering|SetVisibility _pointlight false false)
      (Utilities|FlowControl|Delay (Variables|Default|GetDelayTime))
      (Rendering|SetVisibility _pointlight true false)
      (Utilities|FlowControl|Delay 1.0)
      (bind _result (Math|Integer|IncrementInt (Variables|Default|GetCounter))
        (:%20%20
          (bind _output_get (Variables|Default|SetCounter _result))
          (goto _label))))))

(event EventTick
  (params (DeltaSeconds :type Float%20%28single-precision%29))
  (Development|PrintString (Utilities|String|ToString(Integer) (stale EventBeginPlay _output_get)) true true "(R=0.000000,G=0.660000,B=1.000000,A=1.000000)" 0.0))

(fn ConstructionScript
  (Rendering|Components|Light|SetLightColor (Variables|Default|GetPointLight) (Variables|Default|GetColor) true))